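; Short-lived melee hitbox actor that deals fixed damage, attributed to the player controller at index 1.
; Its Sphere overlap skips that player's own pawn, applies damage to any other overlapping actor with that controller as instigator, then destroys itself.
; If nothing is hit, it destroys itself after a brief delay from BeginPlay.
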(event OnComponentBeginOverlap(Sphere)
  (params (OverlappedComponent :type Primitive%20Component%20Object%20Reference) (OtherActor :type Actor%20Object%20Reference) (OtherComp :type Primitive%20Component%20Object%20Reference) (OtherBodyIndex :type Integer) (bFromSweep :type Boolean) (SweepResult :type Hit%20Result%20Structure%20%28by%20ref%29))
  (bind _returnvalue (Game|GetPlayerController 1))
  (if (not (== (Pawn|GetControlledPawn _returnvalue) (Components|GetOwner OtherComp)))
    (Game|Damage|ApplyDamage OtherActor 15.0 _returnvalue self)
    (Actor|DestroyActor)))

(event EventBeginPlay
  (Utilities|FlowControl|Delay 0.1)
  (Actor|DestroyActor))

(event EventTick
  (params (DeltaSeconds :type Float%20%28single-precision%29)))

(fn ConstructionScript)