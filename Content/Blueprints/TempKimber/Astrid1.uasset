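; Paper2D player character Kimber for a Smash-style platform fighter, with ground and air attacks, projectiles, an air dash and swap animation.
; Attack inputs check IsJumping, play a flipbook, then use timed delays to spawn Melee actors at two arrows.
; Tick picks flipbooks from movement and State, and respawns the character after falls.
; Damage accumulates in Healthperc and scales knockback away from the attacker; hit stun runs on only one side.
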(event Custom|UpdateAnimation1
  ;[1 1 1] General Animations
  (if (not (Variables|Default|Getishit))
    (if (Variables|Default|GetisIdle)
      (Sprite|SetFlipbook (Variables|Default|GetSprite) (select (> (Math|Vector|VectorLength (Math|Conversions|ToVector(Float) (.x (Transformation|GetVelocity)))) 0.0) "/Game/2DSideScroller/Sprites/Kimber/KimberRun/KimberRun.KimberRun" "/Game/2DSideScroller/Sprites/Kimber/Kimber_Idle/KimberIdle.KimberIdle"))
      (Variables|Default|SetisIdle false))
    (Math|Float|CompareFloat (.X (Math|Vector|BreakVector (Variables|/Script/Engine.MovementComponent|GetVelocity (Variables|Character|GetCharacterMovement)))) 0.0
      (:>
        (Pawn|SetControlRotation (Pawn|GetController) (Math|Rotator|MakeRotator 0.0 0.0 0.0)))
      (:<
        (Pawn|SetControlRotation (Pawn|GetController) (Math|Rotator|MakeRotator 0.0 0.0 1.8e+02))))
    (switch Utilities|FlowControl|Switch|SwitchonChar_States (Variables|Default|GetState)
      (:NewEnumerator0
        (if (not (Variables|Default|GetisJumping))
          (Variables|Default|SetisIdle true)
          (Sprite|SetFlipbook (Variables|Default|GetSprite) (select (> (Math|Vector|VectorLength (Math|Conversions|ToVector(Float) (.x (Transformation|GetVelocity)))) 0.0) "/Game/2DSideScroller/Sprites/Kimber/KimberRun/KimberRun.KimberRun" "/Game/2DSideScroller/Sprites/Kimber/Kimber_Idle/KimberIdle.KimberIdle"))))
      (:NewEnumerator2
        (Sprite|SetFlipbook (Variables|Default|GetSprite) "/Game/2DSideScroller/Sprites/Kimber/KimberJump/KimberJump.KimberJump"))
      (:NewEnumerator4
        (Sprite|SetFlipbook (Variables|Default|GetSprite) "/Game/2DSideScroller/Sprites/Kimber/KimberHit/KimberHit.KimberHit")
        (Utilities|FlowControl|Delay 1.0))
      (:NewEnumerator7
        (Sprite|SetFlipbook (Variables|Default|GetSprite) "/Game/2DSideScroller/Sprites/Kimber/KimberHit/KimberHit.KimberHit")))))

(event Custom|Spawn
  (bind _sprite (Variables|Default|GetSprite))
  (Input|SetIgnoreMoveInput (Pawn|GetController) true)
  (Audio|SpawnSoundAttached "/Game/Sounds/Game_Sounds/swap.swap" _sprite "None" "0, 0, 0" "0, 0, 0" "KeepRelativeOffset" false 1.0 1.0 0.0 0 0)
  (Variables|Default|SetisIdle false)
  (Sprite|SetFlipbook _sprite "/Game/2DSideScroller/Sprites/Kimber/KimberSwap/KimberSwap.KimberSwap")
  (Input|ResetIgnoreMoveInput (Pawn|GetController)))

(event EventBeginPlay)

(event Game|Damage|EventAnyDamage
  (params (Damage :type Float%20%28single-precision%29) (DamageType :type Damage%20Type%20Object%20Reference) (InstigatedBy :type Controller%20Object%20Reference) (DamageCauser :type Actor%20Object%20Reference))
  (Variables|Default|Sethealthperc (+ Damage (Variables|Default|Gethealthperc)))
  (if (<= (- (.x (Transformation|GetActorLocation DamageCauser)) (.x (Transformation|GetActorLocation))) 0.0)
    (Character|LaunchCharacter (Math|Vector|MakeVector (* Damage (Variables|Default|Gethealthperc)) 0.0 2e+02) true true)
    (else
      (Character|LaunchCharacter (Math|Vector|MakeVector (* -1.0 (* Damage (Variables|Default|Gethealthperc))) 0.0 2e+02) true true)
      (Variables|Default|Setishit true)
      (Input|SetIgnoreMoveInput (Pawn|GetController) true)
      (Sprite|SetFlipbook (Variables|Default|GetSprite) "/Game/2DSideScroller/Sprites/Kimber/KimberHit/KimberHit.KimberHit")
      (Utilities|FlowControl|Delay 0.2)
      (Input|ResetIgnoreMoveInput (Pawn|GetController))
      (Variables|Default|Setishit false))))

(event EventTick
  (params (DeltaSeconds :type Float%20%28single-precision%29))
  (CallFunction|UpdateAnimation1)
  (if (< (.z (Transformation|GetActorLocation)) -1e+03)
    (Variables|/Script/Engine.MovementComponent|SetVelocity (Variables|Character|GetCharacterMovement) "0, 0, 0")
    (Transformation|SetActorLocation "-254.055511,1.776047,675.000000" false false)
    (Variables|Default|Sethealthperc 0.0)))

(event EventOnLanded
  (params (Hit :type Hit%20Result%20Structure%20%28by%20ref%29))
  (Variables|Default|SetcanAirDash true)
  (Variables|Default|SetisIdle true)
  (Variables|Default|SetisJumping false))

(event Input|ActionEvents|InputActionJump
  (params (Key :type Key%20Structure))
  (bind _sprite (Variables|Default|GetSprite))
  ;[1 1 1] General Animations
  (:Pressed
    (Variables|Default|SetisJumping true)
    (Variables|Default|SetisIdle false)
    (if (not (Variables|Default|GetisDashing))
      (Character|Jump)
      (Sprite|SetFlipbook _sprite "/Game/2DSideScroller/Sprites/Kimber/KimberJump/KimberJump.KimberJump")
      (Audio|SpawnSoundAttached "/Game/Sounds/Game_Sounds/snd_se_Falco_jump02.snd_se_Falco_jump02" _sprite "None" "0, 0, 0" "0, 0, 0" "KeepRelativeOffset" false 1.0 1.0 0.0 0 0)))
  (:Released
    (Variables|Default|SetisJumping true)
    (Variables|Default|SetisIdle false)
    (if (not (Variables|Default|GetisDashing))
      (Character|StopJumping)
      (Variables|Default|SetState "NewEnumerator0"))))

(event Input|ActionEvents|InputActionSpecial
  (params (Key :type Key%20Structure))
  (bind _returnvalue (Pawn|GetControlRotation :!class /Script/Engine.Pawn))
  (bind _sprite (Variables|Default|GetSprite))
  (:Pressed
    ;[1 1 1] Air Projectile on E press
    (if (Variables|Default|GetisJumping)
      (Variables|Default|SetisJumping true)
      (Sprite|SetFlipbook _sprite "/Game/2DSideScroller/Sprites/Kimber/KimberNSpecialAir/KimberNSpecialAir.KimberNSpecialAir")
      (Audio|SpawnSoundAttached "/Game/Sounds/Game_Sounds/snd_se_Falco_Special_C2_N03.snd_se_Falco_Special_C2_N03" _sprite "None" "0, 0, 0" "0, 0, 0" "KeepRelativeOffset" false 1.0 1.0 0.0 0 0)
      (Utilities|FlowControl|Delay 0.4)
      (Variables|Default|SetisJumping false)
      (Game|SpawnActorfromClass "/Game/Blueprints/projectile1.projectile1_C" (Math|Transform|MakeTransform (+ (Transformation|GetActorLocation) (* (Math|Vector|GetForwardVector _returnvalue) 25.0)) _returnvalue) "Undefined" 0 0)
      (Audio|SpawnSoundAttached "/Game/Sounds/Game_Sounds/snd_se_Falco_Special_C3_N01.snd_se_Falco_Special_C3_N01" _sprite "None" "0, 0, 0" "0, 0, 0" "KeepRelativeOffset" false 1.0 1.0 0.0 0 0))))

(event Input|ActionEvents|InputActionUStrong
  (params (Key :type Key%20Structure))
  (bind _sprite (Variables|Default|GetSprite))
  ;[1 1 1] UStrong
  (:Pressed
    (Variables|Default|SetisIdle false)
    (if (not (Variables|Default|GetisJumping))
      (Variables|/Script/Engine.MovementComponent|SetVelocity (Variables|Character|GetCharacterMovement) "0, 0, 0")
      (Input|SetIgnoreMoveInput (Pawn|GetController) true)
      (Sprite|SetFlipbook _sprite "/Game/2DSideScroller/Sprites/Kimber/KimberUStrong/KimberUStrong.KimberUStrong")
      (Utilities|FlowControl|Delay 0.3)
      (Audio|SpawnSoundAttached "/Game/Sounds/Game_Sounds/snd_se_Falco_jump02.snd_se_Falco_jump02" _sprite "None" "0, 0, 0" "0, 0, 0" "KeepRelativeOffset" false 1.0 1.0 0.0 0 0)
      (Audio|SpawnSoundAttached "/Game/Sounds/Game_Sounds/snd_se_Falco_AttackAir_F02.snd_se_Falco_AttackAir_F02" _sprite "None" "0, 0, 0" "0, 0, 0" "KeepRelativeOffset" false 1.0 1.0 0.0 0 0)
      (Game|SpawnActorfromClass "/Game/Blueprints/Melee.Melee_C" (Transformation|GetWorldTransform (Variables|Default|GetArrow1)) "Undefined" 0 0)
      (Game|SpawnActorfromClass "/Game/Blueprints/Melee.Melee_C" (Transformation|GetWorldTransform (Variables|Default|GetArrow2)) "Undefined" 0 0)
      (Utilities|FlowControl|Delay 0.3)
      (Variables|Default|SetisIdle true)
      (Input|ResetIgnoreMoveInput (Pawn|GetController)))))

(event Input|ActionEvents|InputActionBAir
  (params (Key :type Key%20Structure))
  (bind _sprite (Variables|Default|GetSprite))
  ;[1 1 1] BAir
  (:Pressed
    (if (Variables|Default|GetisJumping)
      (Variables|Default|SetisJumping true)
      (Sprite|SetFlipbook _sprite "/Game/2DSideScroller/Sprites/Kimber/aerials/Kimber_Bair/KimberBAir.KimberBAir")
      (Utilities|FlowControl|Delay 0.2)
      (Game|SpawnActorfromClass "/Game/Blueprints/Melee.Melee_C" (Transformation|GetWorldTransform (Variables|Default|GetArrow1)) "Undefined" 0 0)
      (Game|SpawnActorfromClass "/Game/Blueprints/Melee.Melee_C" (Transformation|GetWorldTransform (Variables|Default|GetArrow2)) "Undefined" 0 0)
      (Audio|SpawnSoundAttached "/Game/Sounds/Game_Sounds/snd_se_Falco_AttackAir_F01.snd_se_Falco_AttackAir_F01" _sprite "None" "0, 0, 0" "0, 0, 0" "KeepRelativeOffset" false 1.0 1.0 0.0 0 0)
      (Utilities|FlowControl|Delay 0.3)
      (Variables|Default|SetisJumping false)
      (Input|ResetIgnoreMoveInput (Pawn|GetController)))))

(event Input|ActionEvents|InputActionFair
  (params (Key :type Key%20Structure))
  (bind _sprite (Variables|Default|GetSprite))
  ;[1 1 1] FAir
  (:Pressed
    (if (Variables|Default|GetisJumping)
      (Variables|Default|SetisJumping true)
      (Sprite|SetFlipbook _sprite "/Game/2DSideScroller/Sprites/Kimber/aerials/Kimber_Fair/KimberFAir.KimberFAir")
      (Utilities|FlowControl|Delay 0.25)
      (Game|SpawnActorfromClass "/Game/Blueprints/Melee.Melee_C" (Transformation|GetWorldTransform (Variables|Default|GetArrow1)) "Undefined" 0 0)
      (Game|SpawnActorfromClass "/Game/Blueprints/Melee.Melee_C" (Transformation|GetWorldTransform (Variables|Default|GetArrow2)) "Undefined" 0 0)
      (Audio|SpawnSoundAttached "/Game/Sounds/Game_Sounds/snd_se_item_BeamSword_l.snd_se_item_BeamSword_l" _sprite "None" "0, 0, 0" "0, 0, 0" "KeepRelativeOffset" false 1.0 1.0 0.0 0 0)
      (Utilities|FlowControl|Delay 0.25)
      (Variables|Default|SetisJumping false)
      (Input|ResetIgnoreMoveInput (Pawn|GetController)))))

(event Input|ActionEvents|InputActionUAir
  (params (Key :type Key%20Structure))
  (bind _sprite (Variables|Default|GetSprite))
  ;[1 1 1] UAir
  (:Pressed
    (if (Variables|Default|GetisJumping)
      (Variables|Default|SetisJumping true)
      (Sprite|SetFlipbook _sprite "/Game/2DSideScroller/Sprites/Kimber/aerials/Kimber_UAir/KimberUAir.KimberUAir")
      (Utilities|FlowControl|Delay 0.2)
      (Game|SpawnActorfromClass "/Game/Blueprints/Melee.Melee_C" (Transformation|GetWorldTransform (Variables|Default|GetArrow1)) "Undefined" 0 0)
      (Game|SpawnActorfromClass "/Game/Blueprints/Melee.Melee_C" (Transformation|GetWorldTransform (Variables|Default|GetArrow2)) "Undefined" 0 0)
      (Audio|SpawnSoundAttached "/Game/Sounds/Game_Sounds/snd_se_Falco_AttackAir_F02.snd_se_Falco_AttackAir_F02" _sprite "None" "0, 0, 0" "0, 0, 0" "KeepRelativeOffset" false 1.0 1.0 0.0 0 0)
      (Utilities|FlowControl|Delay 0.3)
      (Variables|Default|SetisJumping false)
      (Input|ResetIgnoreMoveInput (Pawn|GetController)))))

(event Input|ActionEvents|InputActionDair
  (params (Key :type Key%20Structure))
  (bind _sprite (Variables|Default|GetSprite))
  ;[1 1 1] Dair
  (:Pressed
    (if (Variables|Default|GetisJumping)
      (Variables|Default|SetisJumping true)
      (Sprite|SetFlipbook _sprite "/Game/2DSideScroller/Sprites/Kimber/aerials/Kimber_Dair/KimberDAir.KimberDAir")
      (Utilities|FlowControl|Delay 0.2)
      (Game|SpawnActorfromClass "/Game/Blueprints/Melee.Melee_C" (Transformation|GetWorldTransform (Variables|Default|GetArrow1)) "Undefined" 0 0)
      (Game|SpawnActorfromClass "/Game/Blueprints/Melee.Melee_C" (Transformation|GetWorldTransform (Variables|Default|GetArrow2)) "Undefined" 0 0)
      (Audio|SpawnSoundAttached "/Game/Sounds/Game_Sounds/snd_se_Falco_AttackAir_F01.snd_se_Falco_AttackAir_F01" _sprite "None" "0, 0, 0" "0, 0, 0" "KeepRelativeOffset" false 1.0 1.0 0.0 0 0)
      (Utilities|FlowControl|Delay 0.2)
      (Audio|SpawnSoundAttached "/Game/Sounds/Game_Sounds/snd_se_Falco_AttackAir_F02.snd_se_Falco_AttackAir_F02" _sprite "None" "0, 0, 0" "0, 0, 0" "KeepRelativeOffset" false 1.0 1.0 0.0 0 0)
      (Utilities|FlowControl|Delay 0.2)
      (Audio|SpawnSoundAttached "/Game/Sounds/Game_Sounds/snd_se_Falco_AttackAir_F01.snd_se_Falco_AttackAir_F01" _sprite "None" "0, 0, 0" "0, 0, 0" "KeepRelativeOffset" false 1.0 1.0 0.0 0 0)
      (Utilities|FlowControl|Delay 0.3)
      (Variables|Default|SetisIdle false)
      (Input|ResetIgnoreMoveInput (Pawn|GetController)))))

(event Input|ActionEvents|InputActionSpecial
  (params (Key :type Key%20Structure))
  (bind _returnvalue (Pawn|GetControlRotation :!class /Script/Engine.Pawn))
  (bind _sprite (Variables|Default|GetSprite))
  (:Pressed
    ;[1 1 1] Projectile on E press
    (if (not (Variables|Default|GetisJumping))
      (Variables|Default|SetisIdle false)
      (Variables|/Script/Engine.MovementComponent|SetVelocity (Variables|Character|GetCharacterMovement) "0, 0, 0")
      (Sprite|SetFlipbook _sprite "/Game/2DSideScroller/Sprites/Kimber/KimberNSpecial/KimberNSpecial.KimberNSpecial")
      (Audio|SpawnSoundAttached "/Game/Sounds/Game_Sounds/snd_se_Falco_Special_C2_N03.snd_se_Falco_Special_C2_N03" _sprite "None" "0, 0, 0" "0, 0, 0" "KeepRelativeOffset" false 1.0 1.0 0.0 0 0)
      (Utilities|FlowControl|Delay 0.4)
      (Variables|Default|SetisIdle true)
      (Game|SpawnActorfromClass "/Game/Blueprints/projectile1.projectile1_C" (Math|Transform|MakeTransform (+ (Transformation|GetActorLocation) (* (Math|Vector|GetForwardVector _returnvalue) 25.0)) _returnvalue) "Undefined" 0 0)
      (Audio|SpawnSoundAttached "/Game/Sounds/Game_Sounds/snd_se_Falco_Special_C3_N01.snd_se_Falco_Special_C3_N01" _sprite "None" "0, 0, 0" "0, 0, 0" "KeepRelativeOffset" false 1.0 1.0 0.0 0 0))))

(event Input|ActionEvents|InputActionDash
  (params (Key :type Key%20Structure))
  (bind _charactermovement (Variables|Character|GetCharacterMovement))
  (bind _sprite (Variables|Default|GetSprite))
  ;[1 1 1] Dash on Shift (In air)
  (:Pressed
    (if (AI|Components|NavMovement|IsFalling (Variables|Character|GetCharacterMovement))
      (Variables|/Script/Engine.MovementComponent|SetVelocity (Variables|Character|GetCharacterMovement) "0, 0, 0")
      (Variables|Default|SetState "NewEnumerator7")
      (Variables|Default|SetisDashing true)
      (Variables|/Script/Engine.CharacterMovementComponent|SetGroundFriction _charactermovement 0.0)
      (if (AI|Components|NavMovement|IsFalling _charactermovement)
        (if (Variables|Default|GetcanAirDash)
          (if (Variables|Default|GetisDashing)
            (Variables|/Script/Engine.MovementComponent|SetVelocity (Variables|Character|GetCharacterMovement) (Math|Vector|MakeVector (* (.x (Transformation|GetActorForwardVector)) (Variables|Default|GetdashVelocity)) (Variables|Default|Getzero) (Variables|Default|Getzero)))
            (Variables|/Script/Engine.CharacterMovementComponent|SetGravityScale (Variables|Character|GetCharacterMovement) 0.0)
            (Variables|Default|SetcanAirDash false)
            (Variables|Default|SetState "NewEnumerator7")
            (Utilities|FlowControl|Delay 0.4)
            (Variables|/Script/Engine.CharacterMovementComponent|SetGravityScale (Variables|Character|GetCharacterMovement) 3.0)
            (Variables|/Script/Engine.MovementComponent|SetVelocity (Variables|Character|GetCharacterMovement) "0, 0, 0")
            (Variables|Default|SetState "NewEnumerator2")
            (else
              (Variables|/Script/Engine.CharacterMovementComponent|SetGroundFriction (Variables|Character|GetCharacterMovement) 3.0)))))))
  (:Released
    (if (AI|Components|NavMovement|IsFalling (Variables|Character|GetCharacterMovement))
      (Variables|Default|SetState "NewEnumerator7")
      (Sprite|SetFlipbook _sprite "/Game/2DSideScroller/Sprites/Kimber/KimberFSpecial/KimberFSpecial.KimberFSpecial")
      (Variables|Default|SetisDashing false)
      (Variables|/Script/Engine.CharacterMovementComponent|SetGroundFriction _charactermovement 3.0)
      (Audio|SpawnSoundAttached "/Game/Sounds/Game_Sounds/snd_se_Falco_Special_S02.snd_se_Falco_Special_S02" _sprite "None" "0, 0, 0" "0, 0, 0" "KeepRelativeOffset" false 1.0 1.0 0.0 0 0)
      (Audio|SpawnSoundAttached "/Game/Sounds/Game_Sounds/snd_se_Falco_Special_C2_L01.snd_se_Falco_Special_C2_L01" _sprite "None" "0, 0, 0" "0, 0, 0" "KeepRelativeOffset" false 1.0 1.0 0.0 0 0))))

(event Input|ActionEvents|InputActionNair
  (params (Key :type Key%20Structure))
  (bind _sprite (Variables|Default|GetSprite))
  ;[1 1 1] NAir
  (:Pressed
    (if (Variables|Default|GetisJumping)
      (Variables|Default|SetisJumping true)
      (Sprite|SetFlipbook _sprite "/Game/2DSideScroller/Sprites/Kimber/aerials/Kimber_Nair/KimberNair.KimberNair")
      (Utilities|FlowControl|Delay 0.2)
      (Game|SpawnActorfromClass "/Game/Blueprints/Melee.Melee_C" (Transformation|GetWorldTransform (Variables|Default|GetArrow1)) "Undefined" 0 (Game|Player|GetPlayerPawn 0))
      (Game|SpawnActorfromClass "/Game/Blueprints/Melee.Melee_C" (Transformation|GetWorldTransform (Variables|Default|GetArrow2)) "Undefined" 0 (Game|Player|GetPlayerPawn 0))
      (Audio|SpawnSoundAttached "/Game/Sounds/Game_Sounds/snd_se_item_BeamSword_m.snd_se_item_BeamSword_m" _sprite "None" "0, 0, 0" "0, 0, 0" "KeepRelativeOffset" false 1.0 1.0 0.0 0 0)
      (Utilities|FlowControl|Delay 0.3)
      (Variables|Default|SetisJumping false)
      (Input|ResetIgnoreMoveInput (Pawn|GetController)))))

(event Input|ActionEvents|InputActionDStrong
  (params (Key :type Key%20Structure))
  (bind _sprite (Variables|Default|GetSprite))
  ;[1 1 1] DStrong
  (:Pressed
    (Variables|Default|SetisIdle false)
    (if (not (Variables|Default|GetisJumping))
      (Variables|/Script/Engine.MovementComponent|SetVelocity (Variables|Character|GetCharacterMovement) "0, 0, 0")
      (Input|SetIgnoreMoveInput (Pawn|GetController) true)
      (Sprite|SetFlipbook _sprite "/Game/2DSideScroller/Sprites/Kimber/KimberDStrong/KimberDStrong.KimberDStrong")
      (Utilities|FlowControl|Delay 0.15)
      (Audio|SpawnSoundAttached "/Game/Sounds/Game_Sounds/snd_se_item_BeamSword_l.snd_se_item_BeamSword_l" _sprite "None" "0, 0, 0" "0, 0, 0" "KeepRelativeOffset" false 1.0 1.0 0.0 0 0)
      (Utilities|FlowControl|Delay 0.15)
      (Game|SpawnActorfromClass "/Game/Blueprints/Melee.Melee_C" (Transformation|GetWorldTransform (Variables|Default|GetArrow1)) "Undefined" 0 0)
      (Game|SpawnActorfromClass "/Game/Blueprints/Melee.Melee_C" (Transformation|GetWorldTransform (Variables|Default|GetArrow2)) "Undefined" 0 0)
      (Audio|SpawnSoundAttached "/Game/Sounds/Game_Sounds/snd_se_item_BeamSword_l.snd_se_item_BeamSword_l" _sprite "None" "0, 0, 0" "0, 0, 0" "KeepRelativeOffset" false 1.0 1.0 0.0 0 0)
      (Utilities|FlowControl|Delay 0.4)
      (Variables|Default|SetisIdle true)
      (Input|ResetIgnoreMoveInput (Pawn|GetController)))))

(event Input|ActionEvents|InputActionAssist
  (params (Key :type Key%20Structure))
  (bind _sprite (Variables|Default|GetSprite))
  ;[1 1 1] Assist
  (:Pressed
    (Variables|Default|SetisIdle false)
    (if (not (Variables|Default|GetisJumping))
      (Variables|/Script/Engine.MovementComponent|SetVelocity (Variables|Character|GetCharacterMovement) "0, 0, 0")
      (Input|SetIgnoreMoveInput (Pawn|GetController) true)
      (Sprite|SetFlipbook _sprite "/Game/2DSideScroller/Sprites/Kimber/KimberAssist/KimberAssist.KimberAssist")
      (Audio|SpawnSoundAttached "/Game/Sounds/Game_Sounds/snd_se_SZerosuit_Special_C3_N04.snd_se_SZerosuit_Special_C3_N04" _sprite "None" "0, 0, 0" "0, 0, 0" "KeepRelativeOffset" false 1.0 1.0 0.0 0 0)
      (Utilities|FlowControl|Delay 0.7)
      (Game|SpawnActorfromClass "/Game/Blueprints/Melee.Melee_C" (Transformation|GetWorldTransform (Variables|Default|GetArrow1)) "Undefined" 0 0)
      (Game|SpawnActorfromClass "/Game/Blueprints/Melee.Melee_C" (Transformation|GetWorldTransform (Variables|Default|GetArrow2)) "Undefined" 0 0)
      (Audio|SpawnSoundAttached "/Game/Sounds/Game_Sounds/swap.swap" _sprite "None" "0, 0, 0" "0, 0, 0" "KeepRelativeOffset" false 1.0 1.0 0.0 0 0)
      (Audio|SpawnSoundAttached "/Game/Sounds/Game_Sounds/snd_se_item_BeamSword_m.snd_se_item_BeamSword_m" 0 "None" "0, 0, 0" "0, 0, 0" "KeepRelativeOffset" false 1.0 1.0 0.0 0 0)
      (Audio|SpawnSoundAttached "/Game/Sounds/Game_Sounds/snd_se_item_BeamSword_l.snd_se_item_BeamSword_l" _sprite "None" "0, 0, 0" "0, 0, 0" "KeepRelativeOffset" false 1.0 1.0 0.0 0 0)
      (Utilities|FlowControl|Delay 0.32)
      (Variables|Default|SetisIdle true)
      (Input|ResetIgnoreMoveInput (Pawn|GetController)))))

(event Input|ActionEvents|InputActionFStrong
  (params (Key :type Key%20Structure))
  (bind _sprite (Variables|Default|GetSprite))
  ;[1 1 1] FStrong
  (:Pressed
    (Variables|Default|SetisIdle false)
    (if (not (Variables|Default|GetisJumping))
      (Variables|/Script/Engine.MovementComponent|SetVelocity (Variables|Character|GetCharacterMovement) "0, 0, 0")
      (Input|SetIgnoreMoveInput (Pawn|GetController) true)
      (Sprite|SetFlipbook _sprite "/Game/2DSideScroller/Sprites/Kimber/KimberFStrong/KimberFStrong.KimberFStrong")
      (Audio|SpawnSoundAttached "/Game/Sounds/Game_Sounds/snd_se_SZerosuit_Special_C3_N03.snd_se_SZerosuit_Special_C3_N03" _sprite "None" "0, 0, 0" "0, 0, 0" "KeepRelativeOffset" false 1.0 1.0 0.0 0 0)
      (Utilities|FlowControl|Delay 0.4)
      (Game|SpawnActorfromClass "/Game/Blueprints/Melee.Melee_C" (Transformation|GetWorldTransform (Variables|Default|GetArrow1)) "Undefined" 0 0)
      (Game|SpawnActorfromClass "/Game/Blueprints/Melee.Melee_C" (Transformation|GetWorldTransform (Variables|Default|GetArrow2)) "Undefined" 0 0)
      (Audio|SpawnSoundAttached "/Game/Sounds/Game_Sounds/snd_se_SZerosuit_Special_N02.snd_se_SZerosuit_Special_N02" _sprite "None" "0, 0, 0" "0, 0, 0" "KeepRelativeOffset" false 1.0 1.0 0.0 0 0)
      (Audio|SpawnSoundAttached "/Game/Sounds/Game_Sounds/snd_se_item_BeamSword_m.snd_se_item_BeamSword_m" _sprite "None" "0, 0, 0" "0, 0, 0" "KeepRelativeOffset" false 1.0 1.0 0.0 0 0)
      (Utilities|FlowControl|Delay 0.3)
      (Variables|Default|SetisIdle true)
      (Input|ResetIgnoreMoveInput (Pawn|GetController)))))

(event Input|ActionEvents|InputActionJab
  (params (Key :type Key%20Structure))
  (bind _sprite (Variables|Default|GetSprite))
  ;[1 1 1] Jab
  (:Pressed
    (Variables|Default|SetisIdle false)
    (if (not (Variables|Default|GetisJumping))
      (Variables|/Script/Engine.MovementComponent|SetVelocity (Variables|Character|GetCharacterMovement) "0, 0, 0")
      (Input|SetIgnoreMoveInput (Pawn|GetController) true)
      (Sprite|SetFlipbook _sprite "/Game/2DSideScroller/Sprites/Kimber/KimberJab/KimberJabs.KimberJabs")
      (Utilities|FlowControl|Delay 0.08)
      (Game|SpawnActorfromClass "/Game/Blueprints/Melee.Melee_C" (Transformation|GetWorldTransform (Variables|Default|GetArrow1)) "Undefined" 0 0)
      (Game|SpawnActorfromClass "/Game/Blueprints/Melee.Melee_C" (Transformation|GetWorldTransform (Variables|Default|GetArrow2)) "Undefined" 0 0)
      (Audio|SpawnSoundAttached "/Game/Sounds/Game_Sounds/snd_se_item_BeamSword_m1.snd_se_item_BeamSword_m1" _sprite "None" "0, 0, 0" "0, 0, 0" "KeepRelativeOffset" false 1.0 1.0 0.0 0 0)
      (Utilities|FlowControl|Delay 0.17)
      (Variables|Default|SetisIdle true)
      (Input|ResetIgnoreMoveInput (Pawn|GetController)))))

(event Input|AxisEvents|InputAxisMove
  (params (AxisValue :type Float%20%28single-precision%29))
  ;[1 1 1] Running Animation
  (Pawn|Input|AddMovementInput (Math|Vector|GetForwardVector "0, 0, 0") AxisValue false)
  (Variables|Default|SetState "NewEnumerator0"))

(event Input|KeyboardEvents|K
  (params (Key :type Key%20Structure))
  (:Pressed
    (Variables|Default|SetSwapMe true)))

(event Input|KeyboardEvents|L
  (params (Key :type Key%20Structure))
  (:Pressed
    (Actor|DestroyActor)))

(event Input|KeyboardEvents|Period
  (params (Key :type Key%20Structure))
  (bind _sprite (Variables|Default|GetSprite))
  (:Pressed
    (Input|SetIgnoreMoveInput (Pawn|GetController) true)
    (Audio|SpawnSoundAttached "/Game/Sounds/Game_Sounds/swap.swap" _sprite "None" "0, 0, 0" "0, 0, 0" "KeepRelativeOffset" false 1.0 1.0 0.0 0 0)
    (Variables|Default|SetisIdle false)
    (Sprite|SetFlipbook _sprite "/Game/2DSideScroller/Sprites/Kimber/KimberSwap/KimberSwap.KimberSwap")
    (Input|ResetIgnoreMoveInput (Pawn|GetController))))

(event Input|KeyboardEvents|K
  (params (Key :type Key%20Structure))
  (bind _sprite (Variables|Default|GetSprite))
  (:Pressed
    (Input|SetIgnoreMoveInput (Pawn|GetController) true)
    (Audio|SpawnSoundAttached "/Game/Sounds/Game_Sounds/swap.swap" _sprite "None" "0, 0, 0" "0, 0, 0" "KeepRelativeOffset" false 1.0 1.0 0.0 0 0)
    (Variables|Default|SetisIdle false)
    (Sprite|SetFlipbook _sprite "/Game/2DSideScroller/Sprites/Kimber/KimberSwap/KimberSwap.KimberSwap")
    (Input|ResetIgnoreMoveInput (Pawn|GetController))))

(event Input|TouchEvents|InputTouch
  (params (Location :type Vector) (FingerIndex :type ETouchIndex%20Enum))
  (bind _sprite (Variables|Default|GetSprite))
  ;[1 1 1] General Animations
  (:Pressed
    (if (not (Variables|Default|GetisDashing))
      (Character|Jump)
      (Sprite|SetFlipbook _sprite "/Game/2DSideScroller/Sprites/Kimber/KimberJump/KimberJump.KimberJump")
      (Audio|SpawnSoundAttached "/Game/Sounds/Game_Sounds/snd_se_Falco_jump02.snd_se_Falco_jump02" _sprite "None" "0, 0, 0" "0, 0, 0" "KeepRelativeOffset" false 1.0 1.0 0.0 0 0)))
  (:Released
    (if (not (Variables|Default|GetisDashing))
      (Character|StopJumping)
      (Variables|Default|SetState "NewEnumerator0"))))

(fn ConstructionScript
  (bind _charactermovement (Variables|Character|GetCharacterMovement))
  (Variables|Default|SetJumpMaxHoldTime 0.2)
  (Variables|/Script/Engine.CharacterMovementComponent|SetGravityScale _charactermovement 1.5)
  (Variables|/Script/Engine.CharacterMovementComponent|SetGroundFriction _charactermovement 3.0)
  (Variables|/Script/Engine.CharacterMovementComponent|SetJumpZVelocity _charactermovement 3.5e+02)
  (Variables|/Script/Engine.CharacterMovementComponent|SetAirControl _charactermovement 0.3)
  (Variables|/Script/Engine.CharacterMovementComponent|SetAirControlBoostMultiplier _charactermovement 0.0)
  (Variables|/Script/Engine.CharacterMovementComponent|SetAirControlBoostVelocityThreshold _charactermovement 0.0)
  (Variables|/Script/Engine.CharacterMovementComponent|SetMaxAcceleration _charactermovement 2e+03)
  (Sprite|SetFlipbook (Variables|Default|GetSprite) "/Game/2DSideScroller/Sprites/Kimber/Kimber_Idle/KimberIdle.KimberIdle")
  (Variables|Default|SetState "NewEnumerator0"))